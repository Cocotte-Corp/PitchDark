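; Blueprint for a rect light that cycles on and off by itself, starting from the off phase at BeginPlay.
; Two timelines, one per phase, scale TargetIntensity to drive the light's intensity.
; When each timeline finishes, a one-second delay triggers the opposite phase, forming an endless loop.
; A hit on the Box component sets intensity to zero without stopping the timelines.
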(event `self.ReceiveBeginPlay`
  (`self.Light_Off`))

(event `Light_On`
  (bind (_direction _light) (`Timeline|Timeline` :!via `PlayFromStart`)
    (:`Update`
      (`LightComponent.SetIntensity` (`self.RectLight`) (* (`self.TargetIntensity`) _light)))
    (:`Finished`
      (`KismetSystemLibrary.Delay` 1.0)
      (`self.Light_Off`))))

(event `Light_Off`
  (bind (_direction _light) (`Timeline|FadeTrack` :!via `PlayFromStart`)
    (:`Update`
      (`LightComponent.SetIntensity` (`self.RectLight`) (* (`self.TargetIntensity`) _light)))
    (:`Finished`
      (`KismetSystemLibrary.Delay` 1.0)
      (`self.Light_On`))))

(event `self.Box.OnComponentHit`
  (params (HitComponent :type "PrimitiveComponent Object Reference") (OtherActor :type "Actor Object Reference") (OtherComp :type "PrimitiveComponent Object Reference") (NormalImpulse :type "Vector Structure") (Hit :type "HitResult Structure (by ref)"))
  (`LightComponent.SetIntensity` (`self.RectLight`) 0.0))

(fn `UserConstructionScript`)