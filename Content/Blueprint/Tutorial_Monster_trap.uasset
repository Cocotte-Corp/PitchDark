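; Tutorial trap actor that stages a monster ambush and pursuit scene when the player enters its trigger box.
; The first overlap passes a DoOnce before the player pawn check, then spawns three dog NPCs and explosion, fire, fire wall and spark effects at placed location markers.
; It also enables physics on a metal roof part, plays an alert sound and, after a short delay, updates the player's mission to "Run !".
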(event `self.TriggerBox.OnComponentBeginOverlap`
  (params (OverlappedComponent :type "PrimitiveComponent Object Reference") (OtherActor :type "Actor Object Reference") (OtherComp :type "PrimitiveComponent Object Reference") (OtherBodyIndex :type Integer) (bFromSweep :type Boolean) (SweepResult :type "HitResult Structure (by ref)"))
  ;[1 1 1] Player Trigger Box
  (`/Engine/EditorBlueprintResources/StandardMacros.DoOnce` false
    (:`Completed`
      (if (== OtherActor (`GameplayStatics.GetPlayerPawn` 0))
        ;[1 1 1] Spawn Monsters
        (`|SpawnActorFromClass` "/Game/Characters/AI/Child/BP_NPC_Dog2.BP_NPC_Dog2_C" (`KismetMathLibrary.MakeTransform` (`SceneComponent.K2_GetComponentLocation` (`self.monster1loc`))) "AdjustIfPossibleButAlwaysSpawn" "MultiplyWithRoot" null 50.0 null)
        (`|SpawnActorFromClass` "/Game/Characters/AI/Child/BP_NPC_Dog2.BP_NPC_Dog2_C" (`KismetMathLibrary.MakeTransform` (`SceneComponent.K2_GetComponentLocation` (`self.monster2loc`))) "AdjustIfPossibleButAlwaysSpawn" "MultiplyWithRoot" null 50.0 null)
        (`|SpawnActorFromClass` "/Game/Characters/AI/Child/BP_NPC_Dog2.BP_NPC_Dog2_C" (`KismetMathLibrary.MakeTransform` (`SceneComponent.K2_GetComponentLocation` (`self.monster3loc`))) "AdjustIfPossibleButAlwaysSpawn" "MultiplyWithRoot" null 50.0 null)
        ;[1 1 1] Pursuit scene activation fx
        (`|SpawnActorFromClass` "/Game/StarterContent/Blueprints/Blueprint_Effect_Explosion.Blueprint_Effect_Explosion_C" (`KismetMathLibrary.MakeTransform` (`SceneComponent.K2_GetComponentLocation` (`self.explosion location`))) "Undefined" "MultiplyWithRoot" null null)
        (`|SpawnActorFromClass` "/Game/StarterContent/Blueprints/Blueprint_Effect_Fire.Blueprint_Effect_Fire_C" (`KismetMathLibrary.MakeTransform` (`SceneComponent.K2_GetComponentLocation` (`self.fire1loc`))) "Undefined" "MultiplyWithRoot" null null)
        (`|SpawnActorFromClass` "/Game/Blueprint/Blueprint_Effect_wall_fire.Blueprint_Effect_wall_fire_C" (`KismetMathLibrary.MakeTransform` (`SceneComponent.K2_GetComponentLocation` (`self.firewallloc`))) "Undefined" "MultiplyWithRoot" null null)
        (`|SpawnActorFromClass` "/Game/StarterContent/Blueprints/Blueprint_Effect_Sparks.Blueprint_Effect_Sparks_C" (`KismetMathLibrary.MakeTransform` (`SceneComponent.K2_GetComponentLocation` (`self.sparkloc`))) "Undefined" "MultiplyWithRoot" null null)
        (`PrimitiveComponent.SetSimulatePhysics` (`self.metal roof part`) true)
        (`GameplayStatics.PlaySound2D` "/Game/Audio/Monster_alert_cue.Monster_alert_cue" 1.0 1.0 0.0 null null)
        (`KismetSystemLibrary.Delay` 1.0)
        (bind _asbp_player_new_gun (cast `/Game/Blueprint/BP_PlayerNewGun` (`GameplayStatics.GetPlayerCharacter` 0)))
        (`/Game/Blueprint/BP_PlayerNewGun.UpdateMission` _asbp_player_new_gun "Run !")))))

(fn `UserConstructionScript`)