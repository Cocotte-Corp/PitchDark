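; Base interactive pickup for throwables that turns the world item into the player's equipped throwable.
; On TriggerEvent, if the BP_PlayerNewGun character holds no throwable, it spawns EquipedClass at the mesh's BottleSocket transform.
; It stores the spawned BP_Equiped_Parent as ThrowableRef, sets HasThrowable, then destroys itself.
; The spawn only uses the socket's transform with no attachment here, and Interact is empty.
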(event `self.TriggerEvent`
  (bind _asbp_player_new_gun (cast `/Game/Blueprint/BP_PlayerNewGun` (`GameplayStatics.GetPlayerCharacter` 0)))
  (if (not (`/Game/Blueprint/BP_PlayerNewGun.bHasThrowable` _asbp_player_new_gun))
    (bind _returnvalue (`|SpawnActorFromClass` (`self.EquipedClass`) (`SceneComponent.GetSocketTransform` (`Character.Mesh` _asbp_player_new_gun) "BottleSocket" "RTS_World") "Undefined" "MultiplyWithRoot" null null))
    (bind _asbp_equiped_parent (cast `/Game/Blueprint/Interactive/Throwables/BP_Equiped_Parent` _returnvalue))
    (set `/Game/Blueprint/BP_PlayerNewGun.ThrowableRef` _asbp_equiped_parent _asbp_player_new_gun)
    (set `/Game/Blueprint/BP_PlayerNewGun.bHasThrowable` true _asbp_player_new_gun)
    (`self.K2_DestroyActor`)))

(event `/Game/Blueprint/Interface/BPI_Interact.Interact`
  (params (`Character Picking Up` :type "Character Object Reference")))

(fn `UserConstructionScript`
  (`parent.UserConstructionScript`))