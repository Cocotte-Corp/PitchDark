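; Base Blueprint for a throwable item while the player has it equipped, with its collision disabled on construction.
; It caches the BP_PlayerNewGun player on BeginPlay.
; ThrowItem spawns a thrown actor at the player's ThrowableActorClass component, passes its mesh on, and launches the physics sphere at fixed speed along the player-to-spawn-point direction, then destroys the equipped actor.
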(event `self.ReceiveBeginPlay`
  (bind _asbp_player_new_gun (cast `/Game/Blueprint/BP_PlayerNewGun` (`GameplayStatics.GetPlayerCharacter` 0)))
  (set `self.PlayerRef` _asbp_player_new_gun))

(event `ThrowItem`
  (bind _playerref (`self.PlayerRef`))
  (bind _returnvalue (`|SpawnActorFromClass` (`self.Class`) (`KismetMathLibrary.MakeTransform` (`SceneComponent.K2_GetComponentLocation` (`/Game/Blueprint/BP_PlayerNewGun.ThrowableActorClass` _playerref)) (`self.K2_GetActorRotation` _playerref)) "AdjustIfPossibleButAlwaysSpawn" "MultiplyWithRoot" null null))
  (bind _asbp_thrown_parent (cast `/Game/Blueprint/Interactive/Throwables/BP_Thrown_Parent` _returnvalue))
  (`StaticMeshComponent.SetStaticMesh` (`/Game/Blueprint/Interactive/Throwables/BP_Thrown_Parent.mesh` _asbp_thrown_parent) (`self.Mesh`))
  (`PrimitiveComponent.SetPhysicsLinearVelocity` (`/Game/Blueprint/Interactive/Throwables/BP_Thrown_Parent.Sphere` _asbp_thrown_parent) (* (`KismetMathLibrary.GetDirectionUnitVector` (`self.K2_GetActorLocation` (`self.PlayerRef`)) (`self.K2_GetActorLocation` _returnvalue)) 1000.0) false "None")
  (`self.K2_DestroyActor`))

(fn `UserConstructionScript`
  (`self.SetActorEnableCollision` self false))