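; BP_Magazine is an interactable magazine pickup that adds a magazine to the player who picks it up.
; Interact casts the character to BP_PlayerNew, reaches its BPC_Game controller through the PlayerState, and calls AddMagazineToPlayerPC.
; The magazine then destroys itself when running on the server, or otherwise passes itself to the controller's DestroyGunPC for removal.
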(event `/Game/Blueprint/Interface/BPI_Interact.Interact`
  (params (`Character Picking Up` :type "Character Object Reference"))
  (bind _as_bp_player_new_gun (`self.As BP Player New Gun`))
  (bind _asbp_player_new (cast `/Game/Blueprint/BP_PlayerNew` `Character Picking Up`))
  (set `self.As BP Player New Gun` _asbp_player_new)
  (bind _asbpc_game (cast `/Game/Blueprint/Multi/BPC_Game` (`PlayerState.GetPlayerController` (`Pawn.PlayerState` _as_bp_player_new_gun))))
  (`/Game/Blueprint/Multi/BPC_Game.AddMagazineToPlayerPC` _asbpc_game _as_bp_player_new_gun)
  (if (`KismetSystemLibrary.IsServer`)
    (`self.K2_DestroyActor`)
    (else
      (bind _asbpc_game_2 (cast `/Game/Blueprint/Multi/BPC_Game` (`PlayerState.GetPlayerController` (`Pawn.PlayerState` (`self.As BP Player New Gun`)))))
      (`/Game/Blueprint/Multi/BPC_Game.DestroyGunPC` _asbpc_game_2 self))))

(fn `UserConstructionScript`)