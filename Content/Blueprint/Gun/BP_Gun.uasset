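; BP_Gun is the rifle actor that plays the cosmetic side of shooting and reloading on its SkGun skeletal mesh.
; Shoot plays the fire montage, spawns a BP_Casing at the ejection socket set to ignore the player controller when moving, and plays a 2D fire sound.
; Reload plays a sound and the reload montage, then a second sound when the montage completes.
; It contains no projectile, trace, damage or ammo logic.
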(event `/Game/Blueprint/Gun/BPI_Gun.Shoot`
  (`|PlayMontage` (`self.Sk_Gun`) "/Game/Asset/FirstPersonArms/Animations/FP_Rifle_Shoot_Montage.FP_Rifle_Shoot_Montage"
    (:`then`
      (bind _returnvalue (`|SpawnActorFromClass` "/Game/Blueprint/Gun/BP_Casing.BP_Casing_C" (`SceneComponent.GetSocketTransform` (`self.Sk_Gun`) "SOCKET_Ejection" "RTS_World") "AlwaysSpawn" "MultiplyWithRoot" null null))
      (`PrimitiveComponent.IgnoreActorWhenMoving` (`/Game/Blueprint/Gun/BP_Casing.CasingMesh` _returnvalue) (`GameplayStatics.GetPlayerController` 0) true)
      (`GameplayStatics.PlaySound2D` "/Game/MilitaryWeapSilver/Sound/Rifle/Cues/RifleA_Fire_Cue.RifleA_Fire_Cue" 1.0 1.0 0.0 null null))))

(event `/Game/Blueprint/Gun/BPI_Gun.Reload`
  (`GameplayStatics.PlaySound2D` "/Game/MilitaryWeapSilver/Sound/Shotgun/Wavs/Shotgun_Reload03.Shotgun_Reload03" 1.0 1.0 0.0 null null)
  (`|PlayMontage` (`self.Sk_Gun`) "/Game/Asset/AssaultRifle/Animations/AM_FP_WEP_AssaultRifle_Reload.AM_FP_WEP_AssaultRifle_Reload"
    (:`OnCompleted`
      (`GameplayStatics.PlaySound2D` "/Game/Audio/Gun_Reload.Gun_Reload" 1.0 1.0 0.0 null null))))

(fn `UserConstructionScript`)