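; Elevator actor that fakes travel by locking the player in the cage, then moving them to a linked elevator or another level.
; Triggering centers the player, disables movement and closes the door via a timeline that mirrors onto the linked elevator's door.
; A delayed sequence plays ride sound and moving-light animations, then teleports to any linked elevator.
; It finally shows the level-transition widget, or reverses the doors and restores walking.
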(event `PlayLightAnimation`
  (bind _pointlight1 (`self.PointLight1`))
  (bind (_relativelocation_x _relativelocation_y) (`KismetMathLibrary.BreakVector` (`SceneComponent.RelativeLocation` _pointlight1)))
  ;[1 1 1] Light animation
  (`SceneComponent.SetVisibility` _pointlight1 true false)
  (bind (_direction _newtrack_0) (`Timeline|LightAnim` :!via `PlayFromStart`)
    (:`Update`
      (`SceneComponent.K2_SetRelativeLocation` _pointlight1 (`KismetMathLibrary.MakeVector` _relativelocation_x _relativelocation_y _newtrack_0) false false))
    (:`Finished`
      (`SceneComponent.SetVisibility` _pointlight1 false false))))

(event `CloseDoor`
  (bind _door (`self.Door`))
  (bind (_relativelocation_x _relativelocation_y) (`KismetMathLibrary.BreakVector` (`SceneComponent.RelativeLocation` _door)))
  ;[1 1 1] DoorAnimation
  (bind _returnvalue (`GameplayStatics.SpawnSound2D` "/Game/Blueprint/Elevator/resources/sfx/foley-large-mechanical-sliding-steel-gate-closing-359401.foley-large-mechanical-sliding-steel-gate-closing-359401" 1.0 1.0 0.0 null))
  (set `self.NewVar` _returnvalue)
  (set `self.IsInUse?` true)
  (bind (_direction _doortrack) (`Timeline|T_CloseDoor` :!via `PlayFromStart` :!label _label)
    (:`Update`
      (bind _returnvalue_2 (- 90.0 (`KismetMathLibrary.Lerp` -5.0 100.0 _doortrack)))
      (`SceneComponent.K2_SetRelativeLocation` _door (`KismetMathLibrary.MakeVector` _relativelocation_x _relativelocation_y _returnvalue_2) false false)
      (bind _linkedelevator (`self.LinkedElevator`)
        (:`then`
          (bind _door_2 (`/Game/Blueprint/Elevator/BP_Elevator.Door` _linkedelevator))
          (bind (_relativelocation_x_2 _relativelocation_y_2) (`KismetMathLibrary.BreakVector` (`SceneComponent.RelativeLocation` _door_2)))
          (`SceneComponent.K2_SetRelativeLocation` _door_2 (`KismetMathLibrary.MakeVector` _relativelocation_x_2 _relativelocation_y_2 _returnvalue_2) false false))
        (:`else`)))
    (:`Finished`
      (bind _newvar (`self.NewVar`)
        (:`then`
          (`AudioComponent.Stop` _newvar)
          (`ActorComponent.K2_DestroyComponent` _newvar))
        (:`else`
          _))
      (`GameplayStatics.PlaySoundAtLocation` "/Game/Blueprint/Elevator/resources/sfx/SW_Door.SW_Door" (`SceneComponent.K2_GetComponentLocation` (`self.Door`)) (struct) 1.0 1.0 0.0 null null null null)
      (if (`self.IsInUse?`)
        (`self.CallLinkedElevatorEvent`)))))

(event `OpenDoor`
  ;[1 1 1] DoorAnimation
  (bind _returnvalue (`GameplayStatics.SpawnSound2D` "/Game/Blueprint/Elevator/resources/sfx/foley-large-mechanical-sliding-steel-gate-closing-359401.foley-large-mechanical-sliding-steel-gate-closing-359401" 1.0 1.0 0.0 null))
  (set `self.NewVar` _returnvalue)
  (set `self.IsInUse?` false)
  (goto _label :!via `ReverseFromEnd`))

(event `TeleportPlayerToPos`
  ;[1 1 1] Teleport the player to the center of the cage and disable its movements
  (bind _asbp_player_new_gun (cast `/Game/Blueprint/BP_PlayerNewGun` (`GameplayStatics.GetPlayerCharacter` 0)))
  (`self.K2_SetActorLocation` _asbp_player_new_gun (`SceneComponent.K2_GetComponentLocation` (`self.PlayerPos`)) false true)
  (`CharacterMovementComponent.DisableMovement` (`Character.CharacterMovement` _asbp_player_new_gun)))

(event `TriggerElevator`
  ;[1 1 1] Event triggered when button used
  (`self.TeleportPlayerToPos`)
  (`self.CloseDoor`))

(event `CallLinkedElevatorEvent`
  ;[1 1 1] Plays all events for the other elevator
  (bind _returnvalue (`GameplayStatics.SpawnSound2D` "/Game/Blueprint/Elevator/resources/sfx/NewSoundCue.NewSoundCue" 1.0 1.0 0.0 null))
  (`KismetSystemLibrary.Delay` 1.0)
  (`self.PlayLightAnimation`)
  (`KismetSystemLibrary.Delay` 2.0)
  (`self.PlayLightAnimation`)
  (`KismetSystemLibrary.Delay` 2.0)
  (bind _linkedelevator (`self.LinkedElevator`)
    (:`then`
      (`self.PlayLightAnimation`)
      (`KismetSystemLibrary.Delay` 2.0)
      (`AudioComponent.Stop` _returnvalue)
      (`ActorComponent.K2_DestroyComponent` _returnvalue)
      (`self.TeleportPlayerToPos` _linkedelevator))
    (:`else`
      (`AudioComponent.Stop` _returnvalue)
      (`ActorComponent.K2_DestroyComponent` _returnvalue)))
  (bind _linkedlevel (`self.LinkedLevel`)
    (:`then`
      (bind _returnvalue_2 (`|CreateWidget` "/Game/Blueprint/Widget/WBP_TransitionToLevel.WBP_TransitionToLevel_C" null _linkedlevel))
      (`UserWidget.AddToViewport` _returnvalue_2 0))
    (:`else`
      (`self.OpenDoor`)
      (bind _asbp_player_new_gun (cast `/Game/Blueprint/BP_PlayerNewGun` (`GameplayStatics.GetPlayerCharacter` 0)))
      (`CharacterMovementComponent.SetMovementMode` (`Character.CharacterMovement` _asbp_player_new_gun) "MOVE_Walking" 0))))

(fn `UserConstructionScript`)