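; BP_NewElevator is an elevator that moves the player to a linked elevator by teleporting behind closed doors.
; TriggerElevator centers the player in the cage, disables movement and plays a timeline that slides both elevators' doors in sync.
; When closed, it teleports the player into the linked cage, reverses the timeline and restores movement.
; IsInUse stops the reopening from retriggering the transfer; the travel animation is only a debug print.
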(event `CloseDoor`
  (bind _door (`self.Door`))
  (bind (_relativelocation_x _relativelocation_y) (`KismetMathLibrary.BreakVector` (`SceneComponent.RelativeLocation` _door)))
  (set `self.IsInUse?` true)
  (bind (_direction _doortrack) (`Timeline|T_CloseDoor` :!label _label)
    (:`Update`
      (bind _returnvalue (- 150.0 (`KismetMathLibrary.Lerp` 0.0 100.0 _doortrack)))
      (`SceneComponent.K2_SetRelativeLocation` _door (`KismetMathLibrary.MakeVector` _relativelocation_x _relativelocation_y _returnvalue) false false)
      (bind _linkedelevator (`self.LinkedElevator`)
        (:`then`
          (bind _door_2 (`/Game/Blueprint/Elevator/NewElevator/BP_NewElevator.Door` _linkedelevator))
          (bind (_relativelocation_x_2 _relativelocation_y_2) (`KismetMathLibrary.BreakVector` (`SceneComponent.RelativeLocation` _door_2)))
          (`SceneComponent.K2_SetRelativeLocation` _door_2 (`KismetMathLibrary.MakeVector` _relativelocation_x_2 _relativelocation_y_2 _returnvalue) false false))
        (:`else`)))
    (:`Finished`
      (if (`self.IsInUse?`)
        (`self.LinkedElevator`
          (:`then`
            (`self.CallLinkedElevatorEvent`))
          (:`else`))))))

(event `OpenDoor`
  (set `self.IsInUse?` false)
  (goto _label :!via `Reverse`))

(event `TriggerElevator`
  ;[1 1 1] Event triggered when button used
  (`self.TeleportPlayerToPos`)
  (`self.CloseDoor`))

(event `TeleportPlayerToPos`
  ;[1 1 1] Teleport the player to the center of the cage and set his move speed to 0
  (bind _asbp_player (cast `/Game/Blueprint/BP_Player` (`GameplayStatics.GetPlayerCharacter` 0)))
  (`self.K2_SetActorLocation` _asbp_player (`SceneComponent.K2_GetComponentLocation` (`self.PlayerPos`)) false false)
  (set `/Game/Blueprint/BP_Player.CanMove?` false _asbp_player))

(event `CallLinkedElevatorEvent`
  ;[1 1 1] Plays all events for the other elevator
  (`self.TeleportPlayerToPos` (`self.LinkedElevator`))
  (`KismetSystemLibrary.PrintString` "PlayAnimation")
  (`self.OpenDoor`)
  (bind _asbp_player (cast `/Game/Blueprint/BP_Player` (`GameplayStatics.GetPlayerCharacter` 0)))
  (set `/Game/Blueprint/BP_Player.CanMove?` true _asbp_player))

(fn `UserConstructionScript`)