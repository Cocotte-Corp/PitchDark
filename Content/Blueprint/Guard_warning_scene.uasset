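; Guard warning scene actor that plays a one-time scripted event in which a robot guard warns the player, then breaks down.
; The player entering its trigger box starts a warning voice line, followed after a long delay by a Niagara explosion, physics on the guard and a power-down sound.
; It then hides "Guard_warning" tagged actors, sets the "Restore the power" mission and calls DestroyBlockGuard.
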(event `self.TriggerBox.OnComponentBeginOverlap`
  (params (OverlappedComponent :type "PrimitiveComponent Object Reference") (OtherActor :type "Actor Object Reference") (OtherComp :type "PrimitiveComponent Object Reference") (OtherBodyIndex :type Integer) (bFromSweep :type Boolean) (SweepResult :type "HitResult Structure (by ref)"))
  ;[1 1 1] Player Trigger Box
  (`/Engine/EditorBlueprintResources/StandardMacros.DoOnce` false
    (:`Completed`
      (if (== OtherActor (`GameplayStatics.GetPlayerPawn` 0))
        (`GameplayStatics.PlaySound2D` "/Game/Audio/Warning_This_area_is.Warning_This_area_is" 1.0 1.0 0.0 null null)
        (`KismetSystemLibrary.Delay` 19.0)
        (bind _returnvalue (`AddComponent|NODE_AddNiagaraComponent-3` :`RelativeTransform` (`SceneComponent.GetRelativeTransform` (`self.Arrow`))))
        (`NiagaraComponent.SetAsset` _returnvalue "/Game/MixedVFX/Particles/Explosions/NS_ExplosionMidAirSmall.NS_ExplosionMidAirSmall" true)
        (`PrimitiveComponent.SetSimulatePhysics` (`self.Robot_Guard`) true)
        (`GameplayStatics.PlaySound2D` "/Game/StarterContent/Audio/Explosion01.Explosion01" 1.0 1.0 0.0 null null)
        (`KismetSystemLibrary.Delay` 0.4)
        (`GameplayStatics.PlaySound2D` "/Game/Audio/power-down-45784.power-down-45784" 1.0 1.0 0.0 null null)
        (bind _outactors (`GameplayStatics.GetAllActorsWithTag` "Guard_warning"))
        (for _array_element _outactors
          (`self.SetActorHiddenInGame` _array_element true)
          (`KismetSystemLibrary.Delay` 1.0)
          (bind _asbp_player_new_gun (cast `/Game/Blueprint/BP_PlayerNewGun` (`GameplayStatics.GetPlayerCharacter` 0)))
          (`/Game/Blueprint/BP_PlayerNewGun.UpdateMission` _asbp_player_new_gun "Restore the power")
          (`self.DestroyBlockGuard`))))))

(fn `UserConstructionScript`)