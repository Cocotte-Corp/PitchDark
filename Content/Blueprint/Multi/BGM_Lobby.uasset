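; Lobby game mode that tracks connected players and their ready states in a multiplayer lobby.
; Login and logout maintain parallel Players and PlayersReady arrays, matched by index, and copy the player list to BPGS_Lobby.
; SetPlayerReady updates the caller's entry and sends the whole ready array to each player's BPC_Lobby controller.
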(event `self.K2_PostLogin`
  (params (NewPlayer :type "PlayerController Object Reference"))
  (bind _asbps_lobby (cast `/Game/Blueprint/Multi/BPS_Lobby` (`Controller.PlayerState` NewPlayer)))
  (`KismetArrayLibrary.Array_AddUnique` (`self.Players`) _asbps_lobby)
  (`KismetArrayLibrary.Array_Add` (`self.bPlayers Ready`))
  (bind _asbpgs_lobby (cast `/Game/Blueprint/Multi/BPGS_Lobby` (`GameplayStatics.GetGameState`)))
  (set `/Game/Blueprint/Multi/BPGS_Lobby.Player` (`self.Players`) _asbpgs_lobby))

(event `self.K2_OnLogout`
  (params (ExitingController :type "Controller Object Reference"))
  (bind _asbps_lobby (cast `/Game/Blueprint/Multi/BPS_Lobby` (`Controller.PlayerState` ExitingController)))
  (`KismetArrayLibrary.Array_Remove` (`self.bPlayers Ready`) (`KismetArrayLibrary.Array_Find` (`self.Players`) _asbps_lobby))
  (`KismetArrayLibrary.Array_RemoveItem` (`self.Players`) _asbps_lobby)
  (bind _asbpgs_lobby (cast `/Game/Blueprint/Multi/BPGS_Lobby` (`GameplayStatics.GetGameState`)))
  (set `/Game/Blueprint/Multi/BPGS_Lobby.Player` (`self.Players`) _asbpgs_lobby))

(event `Set Player Ready`
  (params (`Player Controller` :type "/Game/Blueprint/Multi/BPC_Lobby Object Reference") (Ready :type Boolean))
  (bind _asbps_lobby (cast `/Game/Blueprint/Multi/BPS_Lobby` (`Controller.PlayerState` `Player Controller`)))
  (`KismetArrayLibrary.Array_Set` (`self.bPlayers Ready`) (`KismetArrayLibrary.Array_Find` (`self.Players`) _asbps_lobby) Ready)
  (for _array_element (`self.Players`)
    (bind _asbpc_lobby (cast `/Game/Blueprint/Multi/BPC_Lobby` (`PlayerState.GetPlayerController` _array_element)))
    (`/Game/Blueprint/Multi/BPC_Lobby.Update Player Ready` _asbpc_lobby (`self.bPlayers Ready`))))

(fn `UserConstructionScript`)