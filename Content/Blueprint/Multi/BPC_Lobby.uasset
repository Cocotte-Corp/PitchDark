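; BPC_Lobby is the lobby player controller, linking each player's lobby widget to ready-state tracking.
; On BeginPlay in L_Lobby, it creates the WBP_Lobby widget and adds it to the viewport.
; ServerUpdatePlayerReady writes readiness to BPS_Lobby and notifies the BGM_Lobby game mode.
; UpdatePlayerReady and UpdatePlayer forward changes to the widget, with player updates delayed by one second.
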(event `self.ReceiveBeginPlay`
  (bind _returnvalue (`GameplayStatics.GetCurrentLevelName` true))
  (if (== _returnvalue "L_Lobby")
    (`self.CreateWidgetLobby`)))

(event `CreateWidgetLobby`
  (bind _returnvalue (`|CreateWidget` "/Game/UI/WBP_Lobby.WBP_Lobby_C" self))
  (bind _output_get (set `self.Ref_WBP_Lobby` _returnvalue))
  (`/Engine/EditorBlueprintResources/StandardMacros.IsValid` _output_get
    (:`Is Valid`
      (`UserWidget.AddToViewport` _output_get 0))))

(event `Server Update Player Ready`
  (params (`Player Ready` :type Boolean))
  (bind _asbps_lobby (cast `/Game/Blueprint/Multi/BPS_Lobby` (`self.PlayerState`)))
  (set `/Game/Blueprint/Multi/BPS_Lobby.bReady` `Player Ready` _asbps_lobby)
  (bind _asbgm_lobby (cast `/Game/Blueprint/Multi/BGM_Lobby` (`GameplayStatics.GetGameMode`)))
  (`/Game/Blueprint/Multi/BGM_Lobby.Set Player Ready` _asbgm_lobby self `Player Ready`))

(event `Update Player Ready`
  (params (`Player Ready` :type "Array of Boolean"))
  (bind _ref_wbp_lobby (`self.Ref_WBP_Lobby`))
  (`/Engine/EditorBlueprintResources/StandardMacros.IsValid` _ref_wbp_lobby
    (:`Is Valid`
      (`/Game/UI/WBP_Lobby.Update Ready Player` _ref_wbp_lobby `Player Ready`))))

(event `Update Player`
  (params (Player :type "Array of /Game/Blueprint/Multi/BPS_Lobby Object Reference"))
  (`KismetSystemLibrary.Delay` 1.0)
  (bind _ref_wbp_lobby (`self.Ref_WBP_Lobby`)
    (:`then`
      (`/Game/UI/WBP_Lobby.Update Player` _ref_wbp_lobby Player))
    (:`else`)))

(fn `UserConstructionScript`)