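; BGM_Game is the multiplayer game mode that acts as a central handler for player weapon and pickup actions.
; PostLogin records each new player's BPS_Game player state in a unique list.
; Custom events destroy gun pickups, forward holster toggles to BP_PlayerNew and increment a player's magazine count.
; AttachToPlayerGM spawns an assault rifle, adds it to equipped weapons, attaches it to the arm's hand socket and toggles the holster.
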(event `self.K2_PostLogin`
  (params (NewPlayer :type "PlayerController Object Reference"))
  (bind _asbps_game (cast `/Game/Blueprint/Multi/BPS_Game` (`Controller.PlayerState` NewPlayer)))
  (`KismetArrayLibrary.Array_AddUnique` (`self.PS_Games`) _asbps_game))

(event `DestroyGunGM`
  (params (GunPickup :type "Actor Object Reference"))
  (`self.K2_DestroyActor` GunPickup))

(event `HolsterGM`
  (params (PC :type "/Game/Blueprint/Multi/BPC_Game Object Reference") (Equiped :type Boolean))
  (bind _asbp_player_new (cast `/Game/Blueprint/BP_PlayerNew` (`Actor.Instigator` PC)))
  (`/Game/Blueprint/BP_PlayerNew.ToggleHolster` _asbp_player_new Equiped))

(event `AttachToPlayerGM`
  (params (Player :type "/Game/Blueprint/BP_PlayerNew Object Reference"))
  (bind _returnvalue (`|SpawnActorFromClass` "/Game/Blueprint/Gun/BP_AssaultRiffle.BP_AssaultRiffle_C" (`KismetMathLibrary.MakeTransform` (0.0 0.0 0.0)) "Undefined" "MultiplyWithRoot" null null))
  (`KismetArrayLibrary.Array_AddUnique` (`/Game/Blueprint/BP_PlayerNew.Equipped_Weapons` Player) _returnvalue)
  (`self.K2_AttachToComponent` _returnvalue (`/Game/Blueprint/BP_PlayerNew.CharacterArm` Player) "ik_hand_gun" "KeepRelative" "KeepRelative" "KeepRelative" true)
  (`/Game/Blueprint/BP_PlayerNew.HolsterToggle` Player))

(event `AddMagazineToPlayer`
  (params (Player :type "/Game/Blueprint/BP_PlayerNew Object Reference"))
  (set `/Game/Blueprint/BP_PlayerNew.Current_Magazine` (+ (`/Game/Blueprint/BP_PlayerNew.Current_Magazine` Player) 1) Player))

(fn `UserConstructionScript`)