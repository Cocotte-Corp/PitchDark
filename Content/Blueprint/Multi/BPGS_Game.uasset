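; BPGS_Game is a multiplayer game state Blueprint that gates a door unlock and handles end-of-session events.
; Tick checks the Slot, Fuel and Scan flags and calls the UnlockDoor dispatcher every frame while all three are true.
; HideWaitWidget hides the first player character's WaitEndHUD.
; DestroySession only opens the main menu level, with no session teardown call.
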(event `self.ReceiveBeginPlay`)

(event `self.ReceiveTick`
  (params (DeltaSeconds :type "Float (single-precision)"))
  (if (and (`self.slot`) (and (`self.fuel`) (`self.scan`)))
    (`self.UnlockDoor`)))

(event `HideWaitWidget`
  (bind _asbp_player_new (cast `/Game/Blueprint/BP_PlayerNew` (`GameplayStatics.GetPlayerCharacter` 0)))
  (`Widget.SetVisibility` (`/Game/Blueprint/BP_PlayerNew.WaitEndHUD` _asbp_player_new) "Hidden"))

(event `DestroySession`
  (`GameplayStatics.OpenLevelBySoftObjectPtr` "/Game/Levels/L_MainMenu.L_MainMenu"))

(fn `UserConstructionScript`)