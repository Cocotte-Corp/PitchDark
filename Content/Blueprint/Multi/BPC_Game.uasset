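; BPC_Game is a player controller for a multiplayer game that relays weapon and attachment requests to the game mode.
; On BeginPlay it caches the BGM_Game game mode, which resolves only on the server.
; Its holster, gun pickup destruction and attach-to-player events forward their arguments to the matching game mode functions when that reference is valid.
; The OnRep handler for the equipped flag is empty.
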(event `self.ReceiveBeginPlay`
  (bind _asbgm_game (cast `/Game/Blueprint/Multi/BGM_Game` (`GameplayStatics.GetGameMode`)))
  (set `self.As BGM Game` _asbgm_game))

(event `HolsterPC`
  (params (Equiped :type Boolean))
  (bind _as_bgm_game (`self.As BGM Game`)
    (:`then`
      (`/Game/Blueprint/Multi/BGM_Game.HolsterGM` _as_bgm_game self Equiped))
    (:`else`)))

(event `DestroyGunPC`
  (params (GunPickup :type "/Game/Blueprint/Gun/BP_GunPickup Object Reference"))
  (bind _as_bgm_game (`self.As BGM Game`)
    (:`then`
      (`/Game/Blueprint/Multi/BGM_Game.DestroyGunGM` _as_bgm_game GunPickup))
    (:`else`)))

(event `AttachToPlayerPC`
  (params (Player :type "/Game/Blueprint/BP_PlayerNewGun Object Reference"))
  (bind _as_bgm_game (`self.As BGM Game`)
    (:`then`
      (`/Game/Blueprint/Multi/BGM_Game.AttachToPlayerGM` _as_bgm_game Player))
    (:`else`)))

(fn `OnRep_bEquiped`)

(fn `UserConstructionScript`)