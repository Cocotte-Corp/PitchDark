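; Jumpscare actor that drops a corpse into the scene when activated.
; Its ActivateJumpscare event spawns a BP_Corpse at the Sphere component's world location with a fixed rotation and plays a collision sound at the same spot.
; Begin play, overlap and tick events are unused, so it does nothing until that event is called.
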(event `self.ActivateJumpscare`
  (bind _returnvalue_location (`KismetMathLibrary.BreakTransform` (`SceneComponent.K2_GetComponentToWorld` (`self.Sphere`))))
  (`|SpawnActorFromClass` "/Game/Blueprint/Jumpscare/BP_Corpse.BP_Corpse_C" (`KismetMathLibrary.MakeTransform` _returnvalue_location (struct :`Pitch` -90.0)) "Undefined" "MultiplyWithRoot" null null)
  (`GameplayStatics.PlaySoundAtLocation` "/Game/Blueprint/Jumpscare/Sfx/SC_Collide.SC_Collide" _returnvalue_location (struct) 1.0 1.0 0.0 null null null null))

(fn `UserConstructionScript`
  (`parent.UserConstructionScript`))