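; BP_jumpscare_Gas is a jumpscare actor that stages a gas leak explosion.
; ActivateJumpscare plays a loud, pitched-down 2D leak explosion sound, then spawns an actor, a positioned explosion sound and a particle explosion at the Sphere component.
; The emitter is destroyed after a short delay.
; The file has no trigger logic of its own, as its overlap, BeginPlay and Tick events are disabled.
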(event `self.ActivateJumpscare`
  (bind (_returnvalue_location _returnvalue_rotation) (`KismetMathLibrary.BreakTransform` (`SceneComponent.K2_GetComponentToWorld` (`self.Sphere`))))
  (`GameplayStatics.PlaySound2D` "/Game/Blueprint/Jumpscare/Sfx/SW_GasLeakExplode.SW_GasLeakExplode" 2.0 0.8 0.0 null null)
  (`|SpawnActorFromClass` "/Game/StarterContent/Blueprints/Blueprint_Effect_Smoke.Blueprint_Effect_Smoke_C" (`KismetMathLibrary.MakeTransform` _returnvalue_location _returnvalue_rotation) "Undefined" "OverrideRootScale" null null)
  (`GameplayStatics.PlaySoundAtLocation` "/Game/Blueprint/Jumpscare/Sfx/SW_GasExplode.SW_GasExplode" _returnvalue_location (struct) 1.0 1.0 0.0 null null null null)
  (bind _returnvalue (`GameplayStatics.SpawnEmitterAtLocation` "/Game/StarterContent/Particles/P_Explosion.P_Explosion" (`SceneComponent.K2_GetComponentLocation` (`self.Sphere`))))
  (`KismetSystemLibrary.Delay` 2.0)
  (`ActorComponent.K2_DestroyComponent` _returnvalue))

(fn `UserConstructionScript`
  (`parent.UserConstructionScript`))