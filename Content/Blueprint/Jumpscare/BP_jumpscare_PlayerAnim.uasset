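; Jumpscare actor that briefly shows a moving skeletal mesh with a scream sound when triggered.
; Calling ActivateJumpscare unhides the mesh, plays SW_Screamer as 2D audio and starts the T_Walk timeline.
; The timeline drives the mesh's relative Y location, then hides it again on finish.
; The file has no trigger logic of its own, as BeginPlay, overlap and Tick are disabled stubs.
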(event `self.ActivateJumpscare`
  (bind _skeletalmesh (`self.SkeletalMesh`))
  (`SceneComponent.SetHiddenInGame` _skeletalmesh false false)
  (`GameplayStatics.PlaySound2D` "/Game/Blueprint/Jumpscare/Sfx/SW_Screamer.SW_Screamer" 1.0 1.0 0.0 null null)
  (bind (_direction _newtrack_0) (`Timeline|T_Walk`)
    (:`Update`
      (`SceneComponent.K2_SetRelativeLocation` (`self.SkeletalMesh`) (`KismetMathLibrary.MakeVector` 0.0 _newtrack_0) false false))
    (:`Finished`
      (`SceneComponent.SetHiddenInGame` _skeletalmesh true false))))

(fn `UserConstructionScript`
  (`parent.UserConstructionScript`))