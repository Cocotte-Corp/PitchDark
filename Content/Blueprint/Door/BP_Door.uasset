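; Door Blueprint that slides its mesh vertically, up to open and down to close.
; OpenDoor and CloseDoor each play their own timeline, offsetting the mesh's current relative Z every update by the curve value times DoorSize, so movement accumulates; comments mark this as temporary.
; Overlapping the Box triggers CloseDoor, while nothing in this graph calls OpenDoor.
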(event `CloseDoor`
  (bind _doormesh (`self.DoorMesh`))
  (bind (_relativelocation_x _relativelocation_y _relativelocation_z) (`KismetMathLibrary.BreakVector` (`SceneComponent.RelativeLocation` _doormesh)))
  ;[1 1 1] Open the door by moving it
  (bind (_direction _dooropening) (`Timeline|Timeline`)
    (:`Update`
      (`SceneComponent.K2_SetRelativeLocation` _doormesh (`KismetMathLibrary.MakeVector` _relativelocation_x _relativelocation_y (- _relativelocation_z (* _dooropening (`self.DoorSize`)))) false false))))

(event `OpenDoor`
  (bind _doormesh (`self.DoorMesh`))
  (bind (_relativelocation_x _relativelocation_y _relativelocation_z) (`KismetMathLibrary.BreakVector` (`SceneComponent.RelativeLocation` _doormesh)))
  ;[1 1 1] Open the door by moving it
  (bind (_direction _dooropening) (`Timeline|T_OpenDoor`)
    (:`Update`
      (`SceneComponent.K2_SetRelativeLocation` _doormesh (`KismetMathLibrary.MakeVector` _relativelocation_x _relativelocation_y (+ _relativelocation_z (* _dooropening (`self.DoorSize`)))) false false))))

(event `self.Box.OnComponentBeginOverlap`
  (params (OverlappedComponent :type "PrimitiveComponent Object Reference") (OtherActor :type "Actor Object Reference") (OtherComp :type "PrimitiveComponent Object Reference") (OtherBodyIndex :type Integer) (bFromSweep :type Boolean) (SweepResult :type "HitResult Structure (by ref)"))
  (`self.CloseDoor`))

(fn `UserConstructionScript`)