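; BP_EndRoomBox is a trigger box that holds players at a room's end until everyone has arrived.
; Box overlaps maintain a count of BP_PlayerNew actors inside, compared against NbPlayer from BPGS_Game.
; Early arrivals that are locally controlled see their WaitEndHUD.
; When the count reaches the total, the game state hides the wait widget and the entering player's camera fades out.
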(event `self.Box.OnComponentBeginOverlap`
  (params (OverlappedComponent :type "PrimitiveComponent Object Reference") (OtherActor :type "Actor Object Reference") (OtherComp :type "PrimitiveComponent Object Reference") (OtherBodyIndex :type Integer) (bFromSweep :type Boolean) (SweepResult :type "HitResult Structure (by ref)"))
  (bind _asbp_player_new (cast `/Game/Blueprint/BP_PlayerNew` OtherActor))
  (bind _asbpgs_game (cast `/Game/Blueprint/Multi/BPGS_Game` (`GameplayStatics.GetGameState`)))
  (bind _output_get (set `self.NbPlayerInZone` (+ (`self.NbPlayerInZone`) 1)))
  (if (>= _output_get (`/Game/Blueprint/Multi/BPGS_Game.NbPlayer` _asbpgs_game))
    (bind _asbpgs_game_2 (cast `/Game/Blueprint/Multi/BPGS_Game` (`GameplayStatics.GetGameState`)))
    (`/Game/Blueprint/Multi/BPGS_Game.HideWaitWidget` _asbpgs_game_2)
    (`/Game/Blueprint/BP_PlayerNew.CameraFadeOut` _asbp_player_new)
    (elif (`Pawn.IsLocallyControlled` _asbp_player_new)
      (`Widget.SetVisibility` (`/Game/Blueprint/BP_PlayerNew.WaitEndHUD` _asbp_player_new) "Visible"))))

(event `self.Box.OnComponentEndOverlap`
  (params (OverlappedComponent :type "PrimitiveComponent Object Reference") (OtherActor :type "Actor Object Reference") (OtherComp :type "PrimitiveComponent Object Reference") (OtherBodyIndex :type Integer))
  (cast `/Game/Blueprint/BP_PlayerNew` OtherActor)
  (set `self.NbPlayerInZone` (- (`self.NbPlayerInZone`) 1)))

(fn `UserConstructionScript`)