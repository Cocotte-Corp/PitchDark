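; Sci-fi door actor that opens once, the first time the player pawn overlaps its TriggerBox.
; The overlap passes a DoOnce, starts the door's open animation, then shows two timed access-request subtitles in sequence using delays.
; A Display_Text event creates a WBP_SubTitle widget for each line and removes it after its duration.
; The Box component is destroyed at the end of the sequence.
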(event `self.triggerBox.OnComponentBeginOverlap`
  (params (OverlappedComponent :type "PrimitiveComponent Object Reference") (OtherActor :type "Actor Object Reference") (OtherComp :type "PrimitiveComponent Object Reference") (OtherBodyIndex :type Integer) (bFromSweep :type Boolean) (SweepResult :type "HitResult Structure (by ref)"))
  ;[1 1 1] Play sound on player trigger
  (if (== OtherActor (`GameplayStatics.GetPlayerPawn` 0))
    (`/Engine/EditorBlueprintResources/StandardMacros.DoOnce` false
      (:`Completed`
        (`SkeletalMeshComponent.PlayAnimation` (`self.Door`) "/Game/Fab/Sci-fi_Door/NRM_OPEN.NRM_OPEN" false)
        (`self.Display_Text` "Requisition of the opening of the door, Z32. " 4.0)
        (`KismetSystemLibrary.Delay` 4.0)
        (`self.Display_Text` "Please wait, Please wait, Please wait. Access granted. Doors opening. " 6.5)
        (`KismetSystemLibrary.Delay` 8.5)
        (`ActorComponent.K2_DestroyComponent` (`self.Box`))))))

(event `Display_Text`
  (params (Text_sub :type Text) (Duration :type "Float (single-precision)"))
  (bind _returnvalue (`|CreateWidget` "/Game/UI/WBP_SubTitle.WBP_SubTitle_C" (`GameplayStatics.GetPlayerController` 0)))
  (`/Game/UI/WBP_SubTitle.Show_text` _returnvalue Text_sub)
  (`UserWidget.AddToViewport` _returnvalue 0)
  (`KismetSystemLibrary.Delay` Duration)
  (`Widget.RemoveFromParent` _returnvalue))

(fn `UserConstructionScript`)