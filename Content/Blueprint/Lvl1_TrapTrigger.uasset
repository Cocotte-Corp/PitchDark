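; Level 1 trap trigger that springs a monster ambush with an alert sound.
; An overlap on the trigger box passes through a DoOnce, then checks that the overlapping actor is the player pawn, so any earlier overlap by another actor uses up the trap.
; On a match it spawns a BP_NPC2 at each of three arrow components and plays the alert as a 2D sound.
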(event `self.TriggerBox.OnComponentBeginOverlap`
  (params (OverlappedComponent :type "PrimitiveComponent Object Reference") (OtherActor :type "Actor Object Reference") (OtherComp :type "PrimitiveComponent Object Reference") (OtherBodyIndex :type Integer) (bFromSweep :type Boolean) (SweepResult :type "HitResult Structure (by ref)"))
  ;[1 1 1] Player Trigger Box
  (`/Engine/EditorBlueprintResources/StandardMacros.DoOnce` false
    (:`Completed`
      (if (== OtherActor (`GameplayStatics.GetPlayerPawn` 0))
        ;[1 1 1] Spawn Monsters
        (`|SpawnActorFromClass` "/Game/Characters/AI/BP_NPC2.BP_NPC2_C" (`KismetMathLibrary.MakeTransform` (`SceneComponent.K2_GetComponentLocation` (`self.Arrow`))) "Undefined" "MultiplyWithRoot" null 100.0 null)
        (`|SpawnActorFromClass` "/Game/Characters/AI/BP_NPC2.BP_NPC2_C" (`KismetMathLibrary.MakeTransform` (`SceneComponent.K2_GetComponentLocation` (`self.Arrow1`))) "Undefined" "MultiplyWithRoot" null 100.0 null)
        (`|SpawnActorFromClass` "/Game/Characters/AI/BP_NPC2.BP_NPC2_C" (`KismetMathLibrary.MakeTransform` (`SceneComponent.K2_GetComponentLocation` (`self.Arrow2`))) "Undefined" "MultiplyWithRoot" null 100.0 null)
        (`GameplayStatics.PlaySound2D` "/Game/Audio/monster_alert_sound.monster_alert_sound" 1.0 1.0 0.0 null null)))))

(fn `UserConstructionScript`)