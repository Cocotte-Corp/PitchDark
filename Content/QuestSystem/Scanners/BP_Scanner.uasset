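; Paired quest scanner that two players activate together by stepping into the trigger boxes of two linked scanners.
; The first overlap sets both to Waiting, the second starts a self-recalling one-second Delay loop that syncs both progress bars.
; Status changes drive materials and widgets on both, and leaving a box resets the pair.
; Completion disables both triggers, sets the BPGS_Game Scan flag, plays a voice cue and spawns lights.
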(event `UpdateStatus`
  (params (Status :type "/Game/QuestSystem/Scanners/E_ScannerStatus Enum" :default "NewEnumerator0"))
  (bind _cube (`self.Cube`))
  (bind _cube_2 (`self.Cube`))
  (bind _cube_3 (`self.Cube`))
  (bind _cube_4 (`self.Cube`))
  ;[1 1 1] Update the status and color of the scanner
  (bind _output_get (set `self.Status` Status))
  (bind _aswbp_scanner (cast `/Game/QuestSystem/Scanners/WBP_Scanner` (`WidgetComponent.GetWidget` (`self.Widget`))))
  (`/Game/QuestSystem/Scanners/WBP_Scanner.ChangeText` _aswbp_scanner _output_get)
  (switch `/Game/QuestSystem/Scanners/E_ScannerStatus` _output_get
    (:`NewEnumerator0`
      (`PrimitiveComponent.SetMaterial` _cube 2 "/Engine/BasicShapes/BasicShapeMaterial.BasicShapeMaterial")
      (`PrimitiveComponent.SetMaterial` _cube_4 4 "/Engine/BasicShapes/BasicShapeMaterial.BasicShapeMaterial")
      (set `self.active?` false))
    (:`NewEnumerator1`
      (`PrimitiveComponent.SetMaterial` _cube 2 "/Game/QuestSystem/DemoContent/DemoRoom/Materials/M_Button.M_Button")
      (`PrimitiveComponent.SetMaterial` _cube_4 4 "/Game/QuestSystem/DemoContent/DemoRoom/Materials/M_Button.M_Button"))
    (:`NewEnumerator2`
      (`PrimitiveComponent.SetMaterial` _cube_3 2 "/Engine/VREditor/UI/ArrowMaterial.ArrowMaterial")
      (`PrimitiveComponent.SetMaterial` _cube_2 4 "/Engine/VREditor/UI/ArrowMaterial.ArrowMaterial")
      (`SceneComponent.SetVisibility` (`self.Widget1`) true false))
    (:`NewEnumerator3`
      (`PrimitiveComponent.SetMaterial` _cube_3 2 "/Engine/MapTemplates/Materials/BasicAsset03.BasicAsset03")
      (`PrimitiveComponent.SetMaterial` _cube_2 4 "/Engine/MapTemplates/Materials/BasicAsset03.BasicAsset03")
      (`SceneComponent.SetVisibility` (`self.Widget1`) false false)
      (`GameplayStatics.PlaySoundAtLocation` "/Game/QuestSystem/Audio/Cues/Voice_QuestCompleted_Cue.Voice_QuestCompleted_Cue" (`self.K2_GetActorLocation`) (struct) 1.0 1.0 0.0 null null null null)
      (`|SpawnActorFromClass` "/Script/Engine.PointLight" (`KismetMathLibrary.Conv_VectorToTransform` (`SceneComponent.K2_GetComponentLocation` (`self.Arrow`))) "Undefined" "MultiplyWithRoot" null null))))

(event `UpdateAllScanners`
  (params (Status :type "/Game/QuestSystem/Scanners/E_ScannerStatus Enum" :default "NewEnumerator0"))
  ;[1 1 1] Update the status and color of the scanner
  (`self.UpdateStatus` Status)
  (`self.UpdateStatus` (`self.Linked_Scanner`) Status))

(event `Scanning`
  ;[1 1 1] Loading
  (if (`self.active?`)
    (`GameplayStatics.PlaySoundAtLocation` "/Engine/EngineSounds/1kSineTonePing.1kSineTonePing" (`self.K2_GetActorLocation`) (struct) 1.0 1.0 0.0 null null null null)
    (`GameplayStatics.PlaySoundAtLocation` "/Engine/EngineSounds/1kSineTonePing.1kSineTonePing" (`self.K2_GetActorLocation` (`self.Linked_Scanner`)) (struct) 1.0 1.0 0.0 null null null null)
    (if (== (`self.Loading`) 10)
      (`self.LoadingCompleted`)
      (`self.LoadingCompleted` (`self.Linked_Scanner`))
      (`self.UpdateAllScanners` "NewEnumerator3")
      (else
        (`KismetSystemLibrary.Delay` 1.0)
        (bind _output_get (set `self.Loading` (+ (`self.Loading`) 1)))
        (set `/Game/QuestSystem/Scanners/BP_Scanner.Loading` _output_get (`self.Linked_Scanner`))
        (`self.UpdateProgressBar`)
        (`self.UpdateProgressBar` (`self.Linked_Scanner`))
        (`self.Scanning`)))
    (else
      (`KismetSystemLibrary.PrintString` "Hello"))))

(event `UpdateProgressBar`
  ;[1 1 1] Update progress bar
  (bind _aswbp_scanner_loading_bar (cast `/Game/QuestSystem/Scanners/WBP_Scanner_LoadingBar` (`WidgetComponent.GetWidget` (`self.Widget1`))))
  (`/Game/QuestSystem/Scanners/WBP_Scanner_LoadingBar.UpdateProgressBar` _aswbp_scanner_loading_bar (`KismetMathLibrary.Conv_IntToDouble` (`self.Loading`))))

(event `LoadingCompleted`
  ;[1 1 1] Event when loading si completed
  (`PrimitiveComponent.SetCollisionEnabled` (`self.Box`) "NoCollision")
  (`PrimitiveComponent.SetCollisionEnabled` (`/Game/QuestSystem/Scanners/BP_Scanner.Box` (`self.Linked_Scanner`)) "NoCollision")
  (`KismetSystemLibrary.PrintString` "Completed")
  (bind _asbpgs_game (cast `/Game/Blueprint/Multi/BPGS_Game` (`GameplayStatics.GetGameState`)))
  (set `/Game/Blueprint/Multi/BPGS_Game.scan` true _asbpgs_game))

(event `self.Box.OnComponentEndOverlap`
  (params (OverlappedComponent :type "PrimitiveComponent Object Reference") (OtherActor :type "Actor Object Reference") (OtherComp :type "PrimitiveComponent Object Reference") (OtherBodyIndex :type Integer))
  ;[1 1 1] Event when losing focus
  (`self.UpdateAllScanners` "NewEnumerator0")
  (`self.ResetScanner`)
  (`self.ResetScanner` (`self.Linked_Scanner`)))

(event `ResetScanner`
  ;[1 1 1] Event when losing focus
  (set `self.Loading` 0)
  (`SceneComponent.SetVisibility` (`self.Widget1`) false false))

(event `self.Box.OnComponentBeginOverlap`
  (params (OverlappedComponent :type "PrimitiveComponent Object Reference") (OtherActor :type "Actor Object Reference") (OtherComp :type "PrimitiveComponent Object Reference") (OtherBodyIndex :type Integer) (bFromSweep :type Boolean) (SweepResult :type "HitResult Structure (by ref)"))
  ;[1 1 1] Event when pressing
  (`GameplayStatics.PlaySoundAtLocation` "/Engine/VREditor/Sounds/UI/Click_on_Button_Cue.Click_on_Button_Cue" (`self.K2_GetActorLocation`) (struct) 1.0 1.0 0.0 null null null null)
  (switch `/Game/QuestSystem/Scanners/E_ScannerStatus` (`self.Status`)
    (:`NewEnumerator0`
      (set `self.active?` true)
      (`self.UpdateAllScanners` "NewEnumerator1")
      (if (`/Game/QuestSystem/Scanners/BP_Scanner.active?` (`self.Linked_Scanner`))
        (`self.Scanning` :!label _label)
        (else
          (`KismetSystemLibrary.PrintString` "Waiting for other player"))))
    (:`NewEnumerator1`
      (set `self.active?` true)
      (`self.UpdateAllScanners` "NewEnumerator2")
      (goto _label))))

(fn `UserConstructionScript`)