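; Interactable checker for the power cell slot puzzle that restores power when the right cells are placed.
; On interact, CheckIfBobines requires all three referenced slots to hold a bobine of the expected color.
; Success plays voice, timed subtitle widgets and power sound once, then sets IsOver and the BPGS_Game Slot flag.
; Failure plays a fail voice throttled by a resetting DoOnce, until the puzzle is over.
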(event `/Game/Blueprint/Interface/BPI_Interact.Interact`
  (params (`Character Picking Up` :type "Character Object Reference"))
  ;[1 1 1] Check if energy cells are placed correctly yes/no
  (bind _isvalid_ (`self.Check If Bobines`))
  (if _isvalid_
    (`KismetSystemLibrary.PrintString` "Valid")
    ;;[1 1 1] Do once to avoid spam
    (`/Engine/EditorBlueprintResources/StandardMacros.DoOnce` false
      (:`Completed`
        (`GameplayStatics.PlaySoundAtLocation` "/Game/QuestSystem/Audio/Voice/Voice_SuccessSlotGame.Voice_SuccessSlotGame" (0.0 0.0 0.0) (struct) 1.0 1.0 0.0 null null null null)
        (`self.Start_vocal`)
        (`/Engine/EditorBlueprintResources/StandardMacros.DoOnce` false
          (:`Completed`
            (`GameplayStatics.PlaySoundAtLocation` "/Game/Audio/powerbackOn.powerbackOn" (`self.K2_GetActorLocation`) (struct) 1.0 1.0 0.0 "/Game/MilitaryWeapSilver/Sound/Attenuation/WeaponHandling_att.WeaponHandling_att" null null null)
            (set `self.IsOver` true)
            (bind _asbpgs_game (cast `/Game/Blueprint/Multi/BPGS_Game` (`GameplayStatics.GetGameState`)))
            (set `/Game/Blueprint/Multi/BPGS_Game.slot` true _asbpgs_game)))))
    (else
      (`KismetSystemLibrary.PrintString` "Invalid")
      (if (not (`self.IsOver`))
        ;;[1 1 1] Play fail, wait to avoid spam
        (`/Engine/EditorBlueprintResources/StandardMacros.DoOnce` false :!label _label
          (:`Completed`
            (`GameplayStatics.PlaySoundAtLocation` "/Game/QuestSystem/Audio/Voice/Voice_FailAttempt.Voice_FailAttempt" (0.0 0.0 0.0) (struct) 1.0 1.0 0.0 null null null null)
            ;;[1 1 1] Comment
            (`KismetSystemLibrary.Delay` 1.0)
            (goto _label :!via `Reset`)))))))

(event `Start_vocal`
  (`self.Display_Text` "Power cell loaded, energy level rising" 3.2)
  (`KismetSystemLibrary.Delay` 3.2)
  (`self.Display_Text` "Redirecting power, door and multiple components back in service" 4.5))

(event `Display_Text`
  (params (Text_sub :type Text) (Duration :type "Float (single-precision)"))
  (bind _returnvalue (`|CreateWidget` "/Game/UI/WBP_SubTitle.WBP_SubTitle_C" (`GameplayStatics.GetPlayerController` 0)))
  (`/Game/UI/WBP_SubTitle.Show_text` _returnvalue Text_sub)
  (`UserWidget.AddToViewport` _returnvalue 0)
  (`KismetSystemLibrary.Delay` Duration)
  (`Widget.RemoveFromParent` _returnvalue))

(fn `Check If Bobines`
  (returns (`IsValid?` :type Boolean))
  (`|ExecutionSequence`
    (:`then_0`
      (bind _slot1 (`self.Slot1`)
        (:`then`
          (bind _stockedbobine (`/Game/QuestSystem/Slots/BP_BobineSlot.StockedBobine` _slot1)
            (:`then`
              (if (not (`|EnumEquality` (`/Game/QuestSystem/Slots/BP_Bobine.Color` _stockedbobine) (`self.Color1`)))
                (`KismetSystemLibrary.PrintString` "setColorSlot")
                (return false)))
            (:`else`
              (return false))))
        (:`else`
          (return false))))
    (:`then_1`
      (bind _slot2 (`self.Slot2`)
        (:`then`
          (bind _stockedbobine_2 (`/Game/QuestSystem/Slots/BP_BobineSlot.StockedBobine` _slot2)
            (:`then`
              (if (not (`|EnumEquality` (`/Game/QuestSystem/Slots/BP_Bobine.Color` _stockedbobine_2) (`self.Color2`)))
                (`KismetSystemLibrary.PrintString` "setColorSlot")
                (return false)))
            (:`else`
              (return false))))
        (:`else`
          (return false))))
    (:`then_2`
      (bind _slot3 (`self.Slot3`)
        (:`then`
          (bind _stockedbobine_3 (`/Game/QuestSystem/Slots/BP_BobineSlot.StockedBobine` _slot3)
            (:`then`
              (if (not (`|EnumEquality` (`/Game/QuestSystem/Slots/BP_Bobine.Color` _stockedbobine_3) (`self.Color3`)))
                (`KismetSystemLibrary.PrintString` "setColorSlot")
                (return false)))
            (:`else`
              (return false))))
        (:`else`
          (return false))))
    (:`then_3`
      (return true))))

(fn `UserConstructionScript`
  (`parent.UserConstructionScript`))