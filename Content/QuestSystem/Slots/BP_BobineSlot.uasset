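; BP_BobineSlot is an interactable slot where the player can deposit a carried bobine.
; On Interact, a BP_PlayerNewGun holding a bobine makes an empty slot spawn a BP_Bobine at its Sphere in the carried color, then clears the player's HasBobine flag.
; If the slot is occupied, it forwards Interact to the stocked bobine instead.
; Players without a bobine get no response from the slot.
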(event `self.Interact`
  (params (`Character Picking Up` :type "Character Object Reference"))
  (bind (_returnvalue_location _returnvalue_rotation) (`KismetMathLibrary.BreakTransform` (`SceneComponent.K2_GetComponentToWorld` (`self.Sphere`))))
  ;[1 1 1] Event interact
  (bind _asbp_player_new_gun (cast `/Game/Blueprint/BP_PlayerNewGun` `Character Picking Up`))
  (if (`/Game/Blueprint/BP_PlayerNewGun.HasBobine?` _asbp_player_new_gun)
    (bind _stockedbobine (`self.StockedBobine`)
      (:`then`
        (`/Game/Blueprint/Interface/BPI_Interact.Interact` _stockedbobine `Character Picking Up`))
      (:`else`
        (bind _returnvalue (`|SpawnActorFromClass` "/Game/QuestSystem/Slots/BP_Bobine.BP_Bobine_C" (`KismetMathLibrary.MakeTransform` _returnvalue_location _returnvalue_rotation) "AdjustIfPossibleButAlwaysSpawn" "MultiplyWithRoot" null (`/Game/Blueprint/BP_PlayerNewGun.BobineColor` _asbp_player_new_gun) (struct) null))
        (set `self.StockedBobine` _returnvalue)
        (set `/Game/Blueprint/BP_PlayerNewGun.HasBobine?` false _asbp_player_new_gun)))))

(fn `UserConstructionScript`
  (`parent.UserConstructionScript`))