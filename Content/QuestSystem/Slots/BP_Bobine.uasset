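; BP_Bobine is a colored bobine pickup (orange, blue or purple) for BP_PlayerNewGun, taken through an Interact event.
; A player without a bobine receives its color and the actor is destroyed.
; A player already holding one swaps colors with it, leaving the pickup in place.
; UpdateColor sets the matching material on the mesh, both after a swap and from the construction script.
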(event `UpdateColor`
  (bind _pickupobject (`self.PickUpObject`))
  ;[1 1 1] Update the color of the bobine
  (switch `/Game/QuestSystem/Slots/E_BobineColor` (`self.Color`)
    (:`NewEnumerator0`
      (`PrimitiveComponent.SetMaterial` _pickupobject 0 "/Engine/TemplateResources/MI_Template_BaseOrange.MI_Template_BaseOrange"))
    (:`NewEnumerator1`
      (`PrimitiveComponent.SetMaterial` _pickupobject 0 "/Game/LevelPrototyping/Materials/MI_Solid_Blue.MI_Solid_Blue"))
    (:`NewEnumerator2`
      (`PrimitiveComponent.SetMaterial` _pickupobject 0 "/DatasmithContent/Materials/AliasReference.AliasReference"))))

(event `/Game/Blueprint/Interface/BPI_Interact.Interact`
  (params (`Character Picking Up` :type "Character Object Reference"))
  (bind _asbp_player_new_gun (cast `/Game/Blueprint/BP_PlayerNewGun` `Character Picking Up`))
  (if (`/Game/Blueprint/BP_PlayerNewGun.HasBobine?` _asbp_player_new_gun)
    (set `self.NewColor` (`/Game/Blueprint/BP_PlayerNewGun.BobineColor` _asbp_player_new_gun))
    (set `/Game/Blueprint/BP_PlayerNewGun.BobineColor` (`self.Color`) _asbp_player_new_gun)
    (set `self.Color` (`self.NewColor`))
    (`self.UpdateColor`)
    (else
      (set `/Game/Blueprint/BP_PlayerNewGun.HasBobine?` true _asbp_player_new_gun)
      (set `/Game/Blueprint/BP_PlayerNewGun.BobineColor` (`self.Color`) _asbp_player_new_gun)
      (`self.K2_DestroyActor`))))

(fn `UserConstructionScript`
  (`parent.UserConstructionScript`)
  (set `self.Color` (`self.NewColor`))
  (`self.UpdateColor`))