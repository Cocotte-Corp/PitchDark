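; Quest actor for a fuel reservoir that the player fills on interact with fuel they are holding.
; FillReservoir moves up to 5 units at a time from the player's FuelQuantity, re-calling itself after a short delay while updating a WBP_Loadingbar widget.
; At 100 units it disables its pickup radius collision, plays an audio cue and sets the Fuel flag on the BPGS_Game game state.
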(event `self.Interact`
  (params (`Character Picking Up` :type "Character Object Reference"))
  (bind _asbp_player_new (cast `/Game/Blueprint/BP_PlayerNew` `Character Picking Up`))
  (`self.FillReservoir` _asbp_player_new))

(event `FillReservoir`
  (params (NewParam :type "/Game/Blueprint/BP_PlayerNew Object Reference"))
  (bind _fuelquantity (`/Game/Blueprint/BP_PlayerNew.FuelQuantity` NewParam))
  (bind _returnvalue (`KismetMathLibrary.FMin` _fuelquantity 5.0))
  (if (and (`/Game/Blueprint/BP_PlayerNew.IsHolding?` NewParam) (!= _fuelquantity 0.0))
    (set `self.FuelCount` (+ (`self.FuelCount`) _returnvalue))
    (set `/Game/Blueprint/BP_PlayerNew.FuelQuantity` (- _fuelquantity _returnvalue) NewParam)
    (bind _aswbp_loadingbar (cast `/Game/QuestSystem/FuelFill/WBP_Loadingbar` (`WidgetComponent.GetWidget` (`self.Widget`))))
    (`/Game/QuestSystem/FuelFill/WBP_Loadingbar.FillBar` _aswbp_loadingbar (/ (`self.FuelCount`) 100.0))
    (if (>= (`self.FuelCount`) 100.0)
      (`KismetSystemLibrary.PrintString` "finito" true true (struct :`R` 1.0 :`G` 0.961659 :`A` 1.0))
      (`PrimitiveComponent.SetCollisionEnabled` (`self.PickUp Radius`) "NoCollision")
      (`GameplayStatics.PlaySoundAtLocation` "/Game/Audio/fuel_entry_audio.fuel_entry_audio" (`self.K2_GetActorLocation`) (struct) 1.0 1.0 0.0 null null null null)
      (bind _asbpgs_game (cast `/Game/Blueprint/Multi/BPGS_Game` (`GameplayStatics.GetGameState`)))
      (set `/Game/Blueprint/Multi/BPGS_Game.fuel` true _asbpgs_game)
      (else
        (`KismetSystemLibrary.PrintString` (`KismetStringLibrary.Conv_DoubleToString` (`self.FuelCount`)))
        (`KismetSystemLibrary.Delay` 0.2)
        (`self.FillReservoir` NewParam)))
    (else
      (`KismetSystemLibrary.PrintString` "not holding or no fuel"))))

(fn `UserConstructionScript`)