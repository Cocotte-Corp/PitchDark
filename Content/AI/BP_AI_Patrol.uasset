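; AI patrol character that walks a loop of four patrol locations and moves toward any pawn it sees.
; GuardPatrol sets a slow walk speed, moves to the indexed location, waits a random interval, then calls itself before incrementing and wrapping the index.
; PawnSensing sightings issue a move to the seen pawn alongside a retriggerable delay that leads nowhere, with no explicit return to patrol.
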(event `self.PawnSensing.OnSeePawn`
  (params (Pawn :type "Pawn Object Reference"))
  (`|ExecutionSequence`
    (:`then_0`
      (`|AIMoveTo` self (0.0 0.0 0.0) Pawn))
    (:`then_1`
      (`KismetSystemLibrary.RetriggerableDelay` 1.0))))

(event `self.ReceiveBeginPlay`
  (`self.GuardPatrol`))

(event `GuardPatrol`
  (set `CharacterMovementComponent.MaxWalkSpeed` 150.0 (`self.CharacterMovement`))
  (`|AIMoveTo` self (`|GetArrayItem` (`self.PatrolLocation`) (`self.Location`)) null
    (:`OnSuccess`
      (`KismetSystemLibrary.Delay` (`KismetMathLibrary.RandomFloatInRange` 1.0 3.0))
      (`self.GuardPatrol`)
      (`/Engine/EditorBlueprintResources/StandardMacros.IncrementInt` (`self.Location`)
        (:`  `
          (if (== (`self.Location`) 4)
            (set `self.Location` 0)))))))

(fn `UserConstructionScript`)