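; BP_NPC2 is a larva monster AI character that damages the player and can be killed.
; Hits are reported as touch-sense stimuli, and the Cover, Advance and Retreat EQS reaction events all crouch.
; Damage triggers Niagara, then a brief halted flinch, or death and delayed destruction if Health was already below zero.
; Attack plays a sound, flags IsAttacking and directly damages player zero without a range check.
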(event `self.ReceiveHit`
  (params (MyComp :type "PrimitiveComponent Object Reference") (Other :type "Actor Object Reference") (OtherComp :type "PrimitiveComponent Object Reference") (bSelfMoved :type Boolean) (HitLocation :type "Vector Structure") (HitNormal :type "Vector Structure") (NormalImpulse :type "Vector Structure") (Hit :type "HitResult Structure (by ref)"))
  ;[1 1 1] Report touch sense stimulus
  (`AISense_Touch.ReportTouchEvent` self Other HitLocation))

(event `self.Cover`
  ;[1 1 1] EQS REACTIONS
  (`self.Crouch`))

(event `self.Advance`
  ;[1 1 1] EQS REACTIONS
  (`self.Crouch`))

(event `self.Retreat`
  ;[1 1 1] EQS REACTIONS
  (`self.Crouch`))

(event `self.ReceiveAnyDamage`
  (params (Damage :type "Float (single-precision)") (DamageType :type "DamageType Object Reference") (InstigatedBy :type "Controller Object Reference") (DamageCauser :type "Actor Object Reference"))
  (bind _mesh (`self.Mesh`))
  ;[1 1 1] Take damages/health system
  (`ActorComponent.Activate` (`self.Niagara`) true)
  (if (>= (`self.Health`) 0.0)
    (set `self.Health` (- (`self.Health`) Damage))
    (set `CharacterMovementComponent.MaxWalkSpeed` 0.0 (`self.CharacterMovement`))
    (`SkeletalMeshComponent.PlayAnimation` _mesh "/Game/Megaspikan/MegaspikanLarvae/Animations/ANIM_MegaspikanLarvae_GetHitFront.ANIM_MegaspikanLarvae_GetHitFront" false)
    (`KismetSystemLibrary.Delay` 1.0)
    (set `CharacterMovementComponent.MaxWalkSpeed` 350.0 (`self.CharacterMovement`))
    (`SkeletalMeshComponent.SetAnimInstanceClass` _mesh "/Game/Animation/ABP_Larvae.ABP_Larvae_C")
    (`GameplayStatics.PlaySoundAtLocation` "/Game/Animation/AI/sfx/ShortMonsterAttackSound.ShortMonsterAttackSound" (`self.K2_GetActorLocation`) (struct) 1.0 1.0 0.0 null null null null)
    (else
      (set `CharacterMovementComponent.MaxWalkSpeed` 0.0 (`self.CharacterMovement`))
      (`GameplayStatics.PlaySoundAtLocation` "/Game/Sound/death/dmg1.dmg1" (`self.K2_GetActorLocation`) (struct) 1.0 1.0 0.0 null null null null)
      (`SkeletalMeshComponent.PlayAnimation` _mesh "/Game/Megaspikan/MegaspikanLarvae/Animations/ANIM_MegaspikanLarvae_Death.ANIM_MegaspikanLarvae_Death" false)
      (`SkeletalMeshComponent.SetPlayRate` _mesh 3.0)
      (`KismetSystemLibrary.Delay` 3.5)
      (`self.K2_DestroyActor`))))

(fn `Attack`
  (returns (`Animation Duration` :type "Float (double-precision)"))
  ;[1 1 1] Attack sound & animation sequence
  (`GameplayStatics.PlaySoundAtLocation` (`self.AttackSound`) (`self.K2_GetActorLocation`) (struct) 1.0 1.0 0.0 null null null null)
  (set `self.bIsAttacking?` true)
  (`GameplayStatics.ApplyDamage` (`GameplayStatics.GetPlayerCharacter` 0) 5.0)
  (return 1.0))

(fn `UserConstructionScript`)