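; BP_Item is a key pickup that triggers a corridor chase when the player takes it.
; Interact sets PickedUp, fires the OnKeyPickedUp dispatcher and returns the item's static mesh to the caller.
; It also starts a short delayed self-destroy and spawns a BP_NPC_Dog running the corridor chase behavior tree at a hardcoded location.
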(event `Destroy item`
  ;[1 1 1] Pick up key & destroy afterwards
  (`KismetSystemLibrary.Delay` 0.2)
  (`self.K2_DestroyActor`))

(event `SpawnMonster`
  ;[1 1 1] Spawn monster for corridor chase sequence
  (if (`self.Picked up`)
    (`AIBlueprintHelperLibrary.SpawnAIFromClass` "/Game/Characters/AI/Child/BP_NPC_Dog.BP_NPC_Dog_C" "/Game/Characters/AI/BT_NPC_corridor_chase.BT_NPC_corridor_chase" (-3250.0 1000.0 240.0) (struct :`Yaw` 80.0) false null)
    (`KismetSystemLibrary.PrintString` "Landed")))

(fn `Interact`
  (returns (`Static mesh` :type "StaticMesh Object Reference"))
  ;[1 1 1] Print out picked up item, destroy object
  (`KismetSystemLibrary.PrintString` "key picked up")
  (set `self.Picked up` true)
  (`self.OnKeyPickedUp` true)
  (`self.Destroy item`)
  (`self.SpawnMonster`)
  (return (`StaticMeshComponent.StaticMesh` (`self.StaticMesh`))))

(fn `UserConstructionScript`)