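; Actor Blueprint for the Megaspikan, a creature built from a main skeletal mesh plus optional skinned part meshes for spawners, shell weak points and jaw weak points.
; On BeginPlay it sets the main mesh as master pose component for every part, so all follow one rig.
; It then makes all those parts visible.
; Overlap, Tick and the construction script hold no logic.
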(event `self.ReceiveBeginPlay`
  ;[1 1 1] Set optional skinned meshes to use main rig
  (`SkinnedMeshComponent.SetLeaderPoseComponent` (`self.SK_Megaspikan_ShellWeakPointRight_B`) (`self.SkeletalMeshComponent`))
  (`SkinnedMeshComponent.SetLeaderPoseComponent` (`self.SK_Megaspikan_SpawnerRight_A`) (`self.SkeletalMeshComponent`))
  (`SkinnedMeshComponent.SetLeaderPoseComponent` (`self.SK_Megaspikan_SpawnerMiddle`) (`self.SkeletalMeshComponent`))
  (`SkinnedMeshComponent.SetLeaderPoseComponent` (`self.SK_Megaspikan_SpawnerLeft_B`) (`self.SkeletalMeshComponent`))
  (`SkinnedMeshComponent.SetLeaderPoseComponent` (`self.SK_Megaspikan_SpawnerLeft_A`) (`self.SkeletalMeshComponent`))
  (`SkinnedMeshComponent.SetLeaderPoseComponent` (`self.SK_Megaspikan_ShellWeakPointRight_C`) (`self.SkeletalMeshComponent`))
  (`SkinnedMeshComponent.SetLeaderPoseComponent` (`self.SK_Megaspikan_JawWeakPointLeft`) (`self.SkeletalMeshComponent`))
  (`SkinnedMeshComponent.SetLeaderPoseComponent` (`self.SK_Megaspikan_ShellWeakPointRight_A`) (`self.SkeletalMeshComponent`))
  (`SkinnedMeshComponent.SetLeaderPoseComponent` (`self.SK_Megaspikan_ShellWeakPointLeft_C`) (`self.SkeletalMeshComponent`))
  (`SkinnedMeshComponent.SetLeaderPoseComponent` (`self.SK_Megaspikan_ShellWeakPointLeft_B`) (`self.SkeletalMeshComponent`))
  (`SkinnedMeshComponent.SetLeaderPoseComponent` (`self.SK_Megaspikan_ShellWeakPointLeft_A`) (`self.SkeletalMeshComponent`))
  (`SkinnedMeshComponent.SetLeaderPoseComponent` (`self.SK_Megaspikan_JawWeakPointRight`) (`self.SkeletalMeshComponent`))
  (`SkinnedMeshComponent.SetLeaderPoseComponent` (`self.SK_Megaspikan_SpawnerRight_B`) (`self.SkeletalMeshComponent`))
  ;[1 1 1] Set visibility of optional skinned meshes
  (`SceneComponent.SetVisibility` (`self.SK_Megaspikan_SpawnerMiddle`) true false)
  (`SceneComponent.SetVisibility` (`self.SK_Megaspikan_SpawnerLeft_B`) true false)
  (`SceneComponent.SetVisibility` (`self.SK_Megaspikan_SpawnerLeft_A`) true false)
  (`SceneComponent.SetVisibility` (`self.SK_Megaspikan_ShellWeakPointRight_C`) true false)
  (`SceneComponent.SetVisibility` (`self.SK_Megaspikan_SpawnerRight_A`) true false)
  (`SceneComponent.SetVisibility` (`self.SK_Megaspikan_ShellWeakPointRight_B`) true false)
  (`SceneComponent.SetVisibility` (`self.SK_Megaspikan_JawWeakPointLeft`) true false)
  (`SceneComponent.SetVisibility` (`self.SK_Megaspikan_ShellWeakPointLeft_C`) true false)
  (`SceneComponent.SetVisibility` (`self.SK_Megaspikan_ShellWeakPointLeft_B`) true false)
  (`SceneComponent.SetVisibility` (`self.SK_Megaspikan_ShellWeakPointLeft_A`) true false)
  (`SceneComponent.SetVisibility` (`self.SK_Megaspikan_JawWeakPointRight`) true false)
  (`SceneComponent.SetVisibility` (`self.SK_Megaspikan_SpawnerRight_B`) true false)
  (`SceneComponent.SetVisibility` (`self.SK_Megaspikan_ShellWeakPointRight_A`) true false))

(fn `UserConstructionScript`)