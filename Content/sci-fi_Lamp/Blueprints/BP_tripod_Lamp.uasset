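; BP_tripod_Lamp is a sci-fi tripod lamp actor with two configurable spot lights, one short-range dynamic and one for GI.
; The construction script applies exposed variables for cone, intensity, radius, indirect lighting and shadows to each light, plus volumetric scattering on the dynamic one.
; Both lights share the same color and temperature variables.
; It also creates a dynamic emissive material on the mesh without setting parameters; the event graph is empty.
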(fn `UserConstructionScript`
  (bind _lit_spotlight_dynamicshortrange_01a (`self.LIT_SpotLight_DynamicShortRange_01A`))
  (bind _lit_spotlight_gi_01a1 (`self.LIT_SpotLight_GI_01A1`))
  (`|ExecutionSequence`
    (:`then_0`
      ;[1 1 1] Dynamic
      (`SpotLightComponent.SetInnerConeAngle` _lit_spotlight_dynamicshortrange_01a (`self.Inner Cone Angle(Dynamic)`))
      (`SpotLightComponent.SetOuterConeAngle` _lit_spotlight_dynamicshortrange_01a (`self.Outer Cone Angle (Dynamic)`))
      (`LightComponent.SetLightColor` _lit_spotlight_dynamicshortrange_01a (`self.Dynamic Light Color`) true)
      (`LightComponent.SetTemperature` _lit_spotlight_dynamicshortrange_01a (`self.Temperature (Dynamic)`))
      (`LightComponent.SetIntensity` _lit_spotlight_dynamicshortrange_01a (`self.Intensity (Dynamic)`))
      (`LocalLightComponent.SetAttenuationRadius` _lit_spotlight_dynamicshortrange_01a (`self.Radius (Dynamic)`))
      (`PrimitiveComponent.CreateDynamicMaterialInstance` (`self.SM_tripod_Lamp`) 1 (`self.Emissive Material`) "None")
      (`LightComponent.SetVolumetricScatteringIntensity` _lit_spotlight_dynamicshortrange_01a (`self.Volumetric scattering Intensity (Dynamic)`))
      (`LightComponent.SetIndirectLightingIntensity` _lit_spotlight_dynamicshortrange_01a (`self.Set Indirect Lighting Intensity (Dynamic)`))
      (`LightComponentBase.SetCastShadows` _lit_spotlight_dynamicshortrange_01a (`self.Cast Shadow (Dynamic)`)))
    (:`then_1`
      ;[1 1 1] GI
      (`SpotLightComponent.SetInnerConeAngle` _lit_spotlight_gi_01a1 (`self.Inner Cone Angle(GI)`))
      (`SpotLightComponent.SetOuterConeAngle` _lit_spotlight_gi_01a1 (`self.Outer Cone Angle(GI)`))
      (`LightComponent.SetLightColor` _lit_spotlight_gi_01a1 (`self.Dynamic Light Color`) true)
      (`LightComponent.SetIntensity` _lit_spotlight_gi_01a1 (`self.Intensity (GI)`))
      (`LightComponent.SetTemperature` _lit_spotlight_gi_01a1 (`self.Temperature (Dynamic)`))
      (`LocalLightComponent.SetAttenuationRadius` _lit_spotlight_gi_01a1 (`self.Radius (GI)`))
      (`LightComponent.SetIndirectLightingIntensity` _lit_spotlight_gi_01a1 (`self.Set Indirect Lighting Intensity (GI)`))
      (`LightComponentBase.SetCastShadows` _lit_spotlight_gi_01a1 (`self.Cast Shadow (GI)`)))))