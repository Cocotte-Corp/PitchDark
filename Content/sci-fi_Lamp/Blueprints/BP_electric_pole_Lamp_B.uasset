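; Electric pole lamp prop (variant B) for a sci-fi lamp set, configured in the construction script with no active runtime logic.
; Two dynamic rect lights share one group of settings, while a separate GI rect light has its own, without a volumetric scattering override.
; All three lights share color and temperature.
; The script also creates a dynamic instance of the emissive material on the pole mesh's second slot, setting no parameters on it.
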(fn `UserConstructionScript`
  (bind _lit_rectlight_dynamic_02a (`self.LIT_RectLight_Dynamic_02A`))
  (bind _lit_rectlight_gi_01a (`self.LIT_RectLight_GI_01A`))
  (bind _lit_rectlight_dynamic_01a (`self.LIT_RectLight_Dynamic_01A`))
  (`|ExecutionSequence`
    (:`then_0`
      ;[1 1 1] Dynamic_Light
      (`LightComponent.SetLightColor` _lit_rectlight_dynamic_01a (`self.Light Color`) true)
      (`LightComponent.SetIntensity` _lit_rectlight_dynamic_01a (`self.Intensity (Dynamic)`))
      (`LocalLightComponent.SetAttenuationRadius` _lit_rectlight_dynamic_01a (`self.Radius (Dynamic)`))
      (`PrimitiveComponent.CreateDynamicMaterialInstance` (`self.SM_electric_pole_Lamp_B`) 1 (`self.Emissive Material`) "None")
      (`LightComponent.SetVolumetricScatteringIntensity` _lit_rectlight_dynamic_01a (`self.Volumetric scattering Intensity (Dynamic)`))
      (`LightComponent.SetIndirectLightingIntensity` _lit_rectlight_dynamic_01a (`self.Indirect Lighting Intensity (Dynamic)`))
      (`LightComponentBase.SetCastShadows` _lit_rectlight_dynamic_01a (`self.Cast Shadow (Dynamic)`))
      (`RectLightComponent.SetBarnDoorAngle` _lit_rectlight_dynamic_01a (`self.Barn Door Angle (Dynamic)`))
      (`LightComponent.SetTemperature` _lit_rectlight_dynamic_01a (`self.Temperature`)))
    (:`then_1`
      (`LightComponent.SetLightColor` _lit_rectlight_dynamic_02a (`self.Light Color`) true)
      (`LightComponent.SetIntensity` _lit_rectlight_dynamic_02a (`self.Intensity (Dynamic)`))
      (`LocalLightComponent.SetAttenuationRadius` _lit_rectlight_dynamic_02a (`self.Radius (Dynamic)`))
      (`LightComponent.SetVolumetricScatteringIntensity` _lit_rectlight_dynamic_02a (`self.Volumetric scattering Intensity (Dynamic)`))
      (`LightComponent.SetIndirectLightingIntensity` _lit_rectlight_dynamic_02a (`self.Indirect Lighting Intensity (Dynamic)`))
      (`LightComponentBase.SetCastShadows` _lit_rectlight_dynamic_02a (`self.Cast Shadow (Dynamic)`))
      (`RectLightComponent.SetBarnDoorAngle` _lit_rectlight_dynamic_02a (`self.Barn Door Angle (Dynamic)`))
      (`LightComponent.SetTemperature` _lit_rectlight_dynamic_02a (`self.Temperature`)))
    (:`then_2`
      ;[1 1 1] GI_Light
      (`LightComponent.SetLightColor` _lit_rectlight_gi_01a (`self.Light Color`) true)
      (`LightComponent.SetIntensity` _lit_rectlight_gi_01a (`self.Intensity (GI)`))
      (`LocalLightComponent.SetAttenuationRadius` _lit_rectlight_gi_01a (`self.Radius (GI)`))
      (`LightComponent.SetIndirectLightingIntensity` _lit_rectlight_gi_01a (`self.Indirect Lighting Intensity (GI)`))
      (`LightComponentBase.SetCastShadows` _lit_rectlight_gi_01a (`self.Cast Shadow (GI)`))
      (`RectLightComponent.SetBarnDoorAngle` _lit_rectlight_gi_01a (`self.Barn Door Angle (GI)`))
      (`LightComponent.SetTemperature` _lit_rectlight_gi_01a (`self.Temperature`)))))