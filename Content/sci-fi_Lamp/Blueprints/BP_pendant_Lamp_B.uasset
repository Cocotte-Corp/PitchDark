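; Configurable sci-fi pendant lamp prop with a mesh, two spot lights (short-range dynamic and GI) and a point light.
; The construction script pushes the exposed variables to each light, covering cones, intensity, radius, shadows and scattering, with color and temperature shared by all three.
; It also creates a dynamic instance of the emissive material on mesh slot 1 without setting parameters on it.
; The event graph has no active logic.
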(fn `UserConstructionScript`
  (bind _lit_pointlight_gi_02a (`self.LIT_PointLight_GI_02A`))
  (bind _lit_spotlight_dynamicshortrange_01a (`self.LIT_SpotLight_DynamicShortRange_01A`))
  (bind _lit_spotlight_gi_01a (`self.LIT_SpotLight_GI_01A`))
  (`|ExecutionSequence`
    (:`then_0`
      ;[1 1 1] Dynamic
      (`SpotLightComponent.SetInnerConeAngle` _lit_spotlight_dynamicshortrange_01a (`self.Inner Cone Angle(Dynamic)`))
      (`SpotLightComponent.SetOuterConeAngle` _lit_spotlight_dynamicshortrange_01a (`self.Outer Cone Angle (Dynamic)`))
      (`LightComponent.SetLightColor` _lit_spotlight_dynamicshortrange_01a (`self.Light Color`) true)
      (`LightComponent.SetTemperature` _lit_spotlight_dynamicshortrange_01a (`self.Temperature`))
      (`LightComponent.SetIntensity` _lit_spotlight_dynamicshortrange_01a (`self.Intensity (Dynamic)`))
      (`LocalLightComponent.SetAttenuationRadius` _lit_spotlight_dynamicshortrange_01a (`self.Radius (Dynamic)`))
      (`PrimitiveComponent.CreateDynamicMaterialInstance` (`self.SM_pendant_Lamp_B`) 1 (`self.Emissive Material`) "None")
      (`LightComponent.SetVolumetricScatteringIntensity` _lit_spotlight_dynamicshortrange_01a (`self.Volumetric scattering Intensity (Dynamic)`))
      (`LightComponent.SetIndirectLightingIntensity` _lit_spotlight_dynamicshortrange_01a (`self.Indirect Lighting Intensity (Dynamic)`))
      (`LightComponentBase.SetCastShadows` _lit_spotlight_dynamicshortrange_01a (`self.Cast Shadow (Dynamic)`)))
    (:`then_1`
      ;[1 1 1] GI
      (`SpotLightComponent.SetInnerConeAngle` _lit_spotlight_gi_01a (`self.Inner Cone Angle(GI)`))
      (`SpotLightComponent.SetOuterConeAngle` _lit_spotlight_gi_01a (`self.Outer Cone Angle(GI)`))
      (`LightComponent.SetLightColor` _lit_spotlight_gi_01a (`self.Light Color`) true)
      (`LightComponent.SetIntensity` _lit_spotlight_gi_01a (`self.Intensity (GI)`))
      (`LightComponent.SetTemperature` _lit_spotlight_gi_01a (`self.Temperature`))
      (`LocalLightComponent.SetAttenuationRadius` _lit_spotlight_gi_01a (`self.Radius (GI)`))
      (`LightComponent.SetIndirectLightingIntensity` _lit_spotlight_gi_01a (`self.Set Indirect Lighting Intensity (GI)`))
      (`LightComponentBase.SetCastShadows` _lit_spotlight_gi_01a (`self.Cast Shadow (GI)`)))
    (:`then_2`
      ;[1 1 1] Point light
      (`LightComponent.SetLightColor` _lit_pointlight_gi_02a (`self.Light Color`) true)
      (`LightComponent.SetIntensity` _lit_pointlight_gi_02a (`self.Intensity (Point light)`))
      (`LocalLightComponent.SetAttenuationRadius` _lit_pointlight_gi_02a (`self.Radius(Point light)`))
      (`LightComponent.SetVolumetricScatteringIntensity` _lit_pointlight_gi_02a (`self.Volumetric scattering Intensity (Point light)`))
      (`LightComponentBase.SetCastShadows` _lit_pointlight_gi_02a (`self.cast shadow (Point light)`))
      (`LightComponent.SetTemperature` _lit_pointlight_gi_02a (`self.Temperature`))
      (`PointLightComponent.SetSoftSourceRadius` _lit_pointlight_gi_02a (`self.Soft Source Radius`)))))