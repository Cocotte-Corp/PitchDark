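; Configurable sci-fi electric pole lamp prop with a static mesh and four point lights.
; The construction script pushes exposed variables to two short-range dynamic lights and two GI lights, which share color and temperature but have separate intensity, radius, shadow, indirect and softness settings.
; Only the dynamic pair receives volumetric scattering, and the lamp mesh's emissive material is set on slot 1.
; The event graph has no runtime logic.
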(fn `UserConstructionScript`
  (bind _lit_pointlight_dynamicshortrange_02a (`self.LIT_PointLight_DynamicShortRange_02A`))
  (bind _lit_pointlight_gi_01a1 (`self.LIT_PointLight_GI_01A1`))
  (bind _lit_pointlight_gi_02a (`self.LIT_PointLight_GI_02A`))
  (bind _lit_pointlight_dynamicshortrange_01a (`self.LIT_PointLight_DynamicShortRange_01A`))
  (`|ExecutionSequence`
    (:`then_0`
      ;[1 1 1] Dynamic
      (`LightComponent.SetLightColor` _lit_pointlight_dynamicshortrange_01a (`self.Light Color`) true)
      (`LightComponent.SetIntensity` _lit_pointlight_dynamicshortrange_01a (`self.Intensity `))
      (`LocalLightComponent.SetAttenuationRadius` _lit_pointlight_dynamicshortrange_01a (`self.Radius `))
      (`PrimitiveComponent.SetMaterial` (`self.SM_electric_pole_Lamp_A`) 1 (`self.Emissive Material`))
      (`LightComponent.SetVolumetricScatteringIntensity` _lit_pointlight_dynamicshortrange_01a (`self.Volumetric scattering Intensity `))
      (`LightComponent.SetIndirectLightingIntensity` _lit_pointlight_dynamicshortrange_01a (`self.Set Indirect Lighting Intensity`))
      (`LightComponentBase.SetCastShadows` _lit_pointlight_dynamicshortrange_01a (`self.Cast Shadow `))
      (`LightComponent.SetTemperature` _lit_pointlight_dynamicshortrange_01a (`self.Temperature`))
      (`PointLightComponent.SetSoftSourceRadius` _lit_pointlight_dynamicshortrange_01a (`self.Soft Source Radius`)))
    (:`then_1`
      (`LightComponent.SetLightColor` _lit_pointlight_dynamicshortrange_02a (`self.Light Color`) true)
      (`LightComponent.SetIntensity` _lit_pointlight_dynamicshortrange_02a (`self.Intensity `))
      (`LocalLightComponent.SetAttenuationRadius` _lit_pointlight_dynamicshortrange_02a (`self.Radius `))
      (`LightComponent.SetVolumetricScatteringIntensity` _lit_pointlight_dynamicshortrange_02a (`self.Volumetric scattering Intensity `))
      (`LightComponent.SetIndirectLightingIntensity` _lit_pointlight_dynamicshortrange_02a (`self.Set Indirect Lighting Intensity`))
      (`LightComponentBase.SetCastShadows` _lit_pointlight_dynamicshortrange_02a (`self.Cast Shadow `))
      (`LightComponent.SetTemperature` _lit_pointlight_dynamicshortrange_02a (`self.Temperature`))
      (`PointLightComponent.SetSoftSourceRadius` _lit_pointlight_dynamicshortrange_02a (`self.Soft Source Radius`)))
    (:`then_2`
      ;[1 1 1] GI
      (`LightComponent.SetLightColor` _lit_pointlight_gi_01a1 (`self.Light Color`) true)
      (`LightComponent.SetIntensity` _lit_pointlight_gi_01a1 (`self.Intensity (GI)`))
      (`LocalLightComponent.SetAttenuationRadius` _lit_pointlight_gi_01a1 (`self.Radius (GI)`))
      (`LightComponentBase.SetCastShadows` _lit_pointlight_gi_01a1 (`self.Cast Shadow (GI)`))
      (`LightComponent.SetTemperature` _lit_pointlight_gi_01a1 (`self.Temperature`))
      (`LightComponent.SetIndirectLightingIntensity` _lit_pointlight_gi_01a1 (`self.Set Indirect Lighting Intensity (GI)`))
      (`PointLightComponent.SetSoftSourceRadius` _lit_pointlight_gi_01a1 (`self.Soft Source Radius (GI)`)))
    (:`then_3`
      (`LightComponent.SetLightColor` _lit_pointlight_gi_02a (`self.Light Color`) true)
      (`LightComponent.SetIntensity` _lit_pointlight_gi_02a (`self.Intensity (GI)`))
      (`LocalLightComponent.SetAttenuationRadius` _lit_pointlight_gi_02a (`self.Radius (GI)`))
      (`LightComponentBase.SetCastShadows` _lit_pointlight_gi_02a (`self.Cast Shadow (GI)`))
      (`LightComponent.SetTemperature` _lit_pointlight_gi_02a (`self.Temperature`))
      (`LightComponent.SetIndirectLightingIntensity` _lit_pointlight_gi_02a (`self.Set Indirect Lighting Intensity (GI)`))
      (`PointLightComponent.SetSoftSourceRadius` _lit_pointlight_gi_02a (`self.Soft Source Radius (GI)`)))))