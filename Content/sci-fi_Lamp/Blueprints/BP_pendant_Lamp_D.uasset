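; A placeable sci-fi pendant lamp Blueprint with a mesh and two configurable point lights, one dynamic short-range and one for GI.
; The construction script pushes exposed variables for intensity, radius, shadows, indirect lighting and soft source radius to each light separately, with color and temperature shared.
; It also sets the mesh's emissive material and the dynamic light's volumetric scattering.
; The event graph holds only disabled stub events, so no runtime logic runs.
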(fn `UserConstructionScript`
  (bind _lit_pointlight_dynamicshortrange_01a (`self.LIT_PointLight_DynamicShortRange_01A`))
  (bind _lit_pointlight_gi_01a1 (`self.LIT_PointLight_GI_01A1`))
  (`|ExecutionSequence`
    (:`then_0`
      ;[1 1 1] Dynamic
      (`LightComponent.SetLightColor` _lit_pointlight_dynamicshortrange_01a (`self.Light Color`) true)
      (`LightComponent.SetIntensity` _lit_pointlight_dynamicshortrange_01a (`self.Intensity `))
      (`LocalLightComponent.SetAttenuationRadius` _lit_pointlight_dynamicshortrange_01a (`self.Radius `))
      (`PrimitiveComponent.SetMaterial` (`self.SM_pendant_Lamp_D`) 0 (`self.Emissive Material`))
      (`LightComponent.SetVolumetricScatteringIntensity` _lit_pointlight_dynamicshortrange_01a (`self.Volumetric scattering Intensity `))
      (`LightComponent.SetIndirectLightingIntensity` _lit_pointlight_dynamicshortrange_01a (`self.Set Indirect Lighting Intensity`))
      (`LightComponentBase.SetCastShadows` _lit_pointlight_dynamicshortrange_01a (`self.Cast Shadow `))
      (`LightComponent.SetTemperature` _lit_pointlight_dynamicshortrange_01a (`self.Temperature`))
      (`PointLightComponent.SetSoftSourceRadius` _lit_pointlight_dynamicshortrange_01a (`self.Soft Source Radius`)))
    (:`then_1`
      ;[1 1 1] GI
      (`LightComponent.SetLightColor` _lit_pointlight_gi_01a1 (`self.Light Color`) true)
      (`LightComponent.SetIntensity` _lit_pointlight_gi_01a1 (`self.Intensity (GI)`))
      (`LocalLightComponent.SetAttenuationRadius` _lit_pointlight_gi_01a1 (`self.Radius (GI)`))
      (`LightComponentBase.SetCastShadows` _lit_pointlight_gi_01a1 (`self.Cast Shadow (GI)`))
      (`LightComponent.SetTemperature` _lit_pointlight_gi_01a1 (`self.Temperature`))
      (`LightComponent.SetIndirectLightingIntensity` _lit_pointlight_gi_01a1 (`self.Set Indirect Lighting Intensity (GI)`))
      (`PointLightComponent.SetSoftSourceRadius` _lit_pointlight_gi_01a1 (`self.Soft Source Radius (GI)`)))))