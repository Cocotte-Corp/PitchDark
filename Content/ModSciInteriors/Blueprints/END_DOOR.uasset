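; END_DOOR is a sci-fi interior door that opens when the game state signals an unlock.
; On BeginPlay it binds its DoorUnlock event to BPGS_Game through BindEventToUnlockDoor.
; When triggered, it activates two SteamDoor effects and plays a timeline that slides DoorSmallA from its closed to open position by lerping its relative location.
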(event `self.ReceiveBeginPlay`
  (bind _asbpgs_game (cast `/Game/Blueprint/Multi/BPGS_Game` (`GameplayStatics.GetGameState`)))
  (add `/Game/Blueprint/Multi/BPGS_Game.UnlockDoor` _asbpgs_game (delegate `DoorUnlock`)))

(event `DoorUnlock`
  (`ActorComponent.Activate` (`self.SteamDoor`) false)
  (`ActorComponent.Activate` (`self.SteamDoor2`) false)
  (bind (_direction _doorposition) (`Timeline|Timeline_0`)
    (:`Update`
      (`SceneComponent.K2_SetRelativeLocation` (`self.Door_Small_A`) (`KismetMathLibrary.VLerp` (`self.DoorClosed`) (`self.DoorOpen`) _doorposition) false false))))

(fn `UserConstructionScript`)